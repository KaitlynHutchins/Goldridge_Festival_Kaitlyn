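; Wandering NPC character that the player can talk to, with a mesh and dialogue row chosen by NPC type.
; It walks to random points around its spawn with random pauses, and box overlaps signal interaction range.
; Interacting stops it, checks the player's minigame leaderboard position to pick dialogue, and saves an upgrade on the default branch.
; Ending interaction resumes wandering or calls minigame start events, which are empty here.
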(event OnComponentBeginOverlap(Box)
  (params (OverlappedComponent :type Primitive%20Component%20Object%20Reference) (OtherActor :type Actor%20Object%20Reference) (OtherComp :type Primitive%20Component%20Object%20Reference) (OtherBodyIndex :type Integer) (bFromSweep :type Boolean) (SweepResult :type Hit%20Result%20Structure%20%28by%20ref%29))
  ;[0.4678 0.05242 0.05138] Interact Widget
  (Class|BPINPCInteract|EnterInteractRange(Message) OtherActor))

(event OnComponentEndOverlap(Box)
  (params (OverlappedComponent :type Primitive%20Component%20Object%20Reference) (OtherActor :type Actor%20Object%20Reference) (OtherComp :type Primitive%20Component%20Object%20Reference) (OtherBodyIndex :type Integer))
  ;[0.4678 0.05242 0.05138] Interact Widget
  (Class|BPINPCInteract|LeaveInteractRange(Message) OtherActor))

(event Custom|WalkRandom
  ;[0.4678 0.05242 0.05138] Walking Random
  (if (Variables|Default|GetShouldNPCWander)
    (if (not (Variables|Default|GetTalking))
      (AI|AIMoveTo self (.RandomLocation (AI|Navigation|GetRandomReachablePointinRadius (Variables|Default|GetSpawnLocation) (Variables|Default|GetWalkDistance) 0 0)) 0 5.0 false
        (:OnSuccess
          _)
        (:OnFail
          _))
      (Utilities|FlowControl|Delay (Math|Random|RandomFloatinRange (Variables|Default|GetRandIntMin) (Variables|Roaming|GetRandIntMax)))
      (CallFunction|WalkRandom))))

(event Custom|BeginShootingMinigame)

(event Custom|BeginBullMinigame)

(event Custom|SetNpcType
  (switch Utilities|FlowControl|Switch|SwitchonE_NPCType (Variables|Default|GetNpcType)
    (:NewEnumerator0
      (Rendering|SetVisibility (Variables|Character|GetMesh) true false)
      (Variables|Default|SetNPCDialogueRow 1))
    (:NewEnumerator1
      (Rendering|SetVisibility (Variables|Character|GetMesh) false false)
      (Rendering|SetVisibility (Variables|Default|GetCowTheyMesh) true false)
      (Variables|Default|SetNPCDialogueRow 18)))
  (CallFunction|WalkRandom))

(event Custom|BeginMinecartMinigame)

(event EventBeginPlay
  (CallFunction|SetNpcType)
  (Variables|/Script/Engine.CharacterMovementComponent|SetMaxWalkSpeed (Variables|Character|GetCharacterMovement) 2e+02)
  (Utilities|FlowControl|Delay (Variables|Default|GetRandIntMin))
  (Variables|Default|SetSpawnLocation (Transformation|GetActorLocation)))

(event EventBegininteract
  (bind _self self)
  ;[1 0.9545 0 0.5] Dialogue Interaction
  (Development|PrintString "Starting Interact in NPC")
  (Components|Movement|StopMovementImmediately (Variables|Character|GetCharacterMovement))
  (Variables|Default|SetTalking true)
  (Development|PrintString "Hello, you are interacting with me!")
  (bind _asbp_first_person_character_kaitlyn (Utilities|Casting|CastToBP_FirstPersonCharacter_Kaitlyn (Game|GetPlayerCharacter 0)))
  (bind _gamedata (Class|BPISaveGame|GetGameData(Message) (Game|GetGameInstance)))
  (bind _minigamedata (CallFunction|GetMinigameData (Variables|Default|GetMinigame) _gamedata))
  (for (_array_element _array_index) (.LeaderboardNames (Utilities|Struct|BreakS_Minigame _minigamedata))
    (if (Utilities|Enum|Equal(Enum) _array_element (Variables|/Game/Kaitlyn_Dev/Blueprints/BP_FirstPersonCharacter_Kaitlyn.BP_FirstPersonCharacter_Kaitlyn_C|GetPlayerName _asbp_first_person_character_kaitlyn))
      (Variables|Default|SetUniqueDialogueConditionsMet (>= _array_index 7))))
  (if (Variables|Default|GetHasUniqueDialogue?)
    (if (Variables|Default|GetUniqueDialogueConditionsMet)
      (Default|DisplayDialogueKaitlyn _asbp_first_person_character_kaitlyn (- (Variables|Default|GetNPCDialogueRow) 1) _self :!label _label)
      (CallFunction|SavePlayerUpgrade (Variables|Default|GetUpgrade) false)
      (else
        (Default|DisplayDialogueKaitlyn _asbp_first_person_character_kaitlyn (- (Variables|Default|GetNPCUniqueDialogueRow) 1) _self)))
    (else
      (goto _label))))

(event EventEndInteract
  ;[1 0.9545 0 0.5] Dialogue Interaction
  (switch Utilities|FlowControl|Switch|SwitchonE_Minigames (Variables|Default|GetMinigame)
    (:NewEnumerator3
      (if (Variables|Default|GetUniqueDialogueConditionsMet) :!label _label
        (Variables|Default|SetUniqueDialogueConditionsMet false))
      (Variables|Default|SetTalking false)
      (Utilities|FlowControl|Delay 0.2)
      (CallFunction|WalkRandom))
    (:NewEnumerator0
      (CallFunction|BeginBullMinigame))
    (:NewEnumerator1
      (CallFunction|BeginMinecartMinigame)
      (goto _label))
    (:NewEnumerator2
      (CallFunction|BeginShootingMinigame))))

(event EventTick
  (params (DeltaSeconds :type Float%20%28single-precision%29))
  ;[0.15 0.15 0.15 0.5] Hopping Code AI
)

(fn ConstructionScript)

(fn DisplayDialogueNPC
  (params (DataTableRowNumber :type Integer) (NPC%20JP :type BP%20JPNPC%20Object%20Reference)))

(fn EnterInteractRange)

(fn GetGameData
  (return 0))

(fn GetMinigameData
  (params (Minigame :type E_Minigames%20Enum :default "NewEnumerator3") (GameData :type BP%20Save%20Game%20Object%20Reference))
  (switch Utilities|FlowControl|Switch|SwitchonE_Minigames Minigame
    (:NewEnumerator0
      (return (Variables|/Game/Shaon/BP_SaveGame.BP_SaveGame_C|GetBullMiniGameSave GameData)))
    (:NewEnumerator1
      (return (Variables|/Game/Shaon/BP_SaveGame.BP_SaveGame_C|GetMinecartMiniGameSave GameData)))
    (:NewEnumerator2
      (return (Variables|/Game/Shaon/BP_SaveGame.BP_SaveGame_C|GetShootingMiniGameSave GameData)))))